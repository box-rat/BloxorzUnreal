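; Parent map Blueprint that builds a tile-based level from the Level1Layout data table.
; GenerateLevel reads each table row's sixteen columns and spawns an Empty, Start or Basic tile on a grid via CoordsToTransform.
; Each tile gets its column/row coordinates and is stored in TileActors, a 2D array made from row structs.
; ClearLevel destroys every Tile actor in the world without resetting that array.
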(event `SpawnEmpty`
  (params (Row :type Integer) (Column :type Integer))
  (bind _transform (`self.CoordsToTransform` Row Column))
  (bind _returnvalue (`|SpawnActorFromClass` "/Game/Tile_Empty.Tile_Empty_C" _transform "Undefined" "MultiplyWithRoot" null null))
  (set `self.GeneratedTile` _returnvalue)
  (bind _output_get (set `/Game/Tile.Coordinates` (`KismetMathLibrary.MakeVector2D` (`KismetMathLibrary.Conv_IntToDouble` (`self.Column Index`)) (`KismetMathLibrary.Conv_IntToDouble` (`self.Row Index`))) (`self.GeneratedTile`) :!label _label))
  (`KismetSystemLibrary.LogString` (`KismetStringLibrary.Concat_StrStr` (`KismetStringLibrary.Conv_Vector2dToString` _output_get) " :: " (`KismetSystemLibrary.GetDisplayName` (`self.GeneratedTile`)))))

(event `SpawnBasic`
  (params (Row :type Integer) (Column :type Integer))
  (bind _transform (`self.CoordsToTransform` Row Column))
  (bind _returnvalue (`|SpawnActorFromClass` "/Game/Tile_Basic.Tile_Basic_C" _transform "Undefined" "MultiplyWithRoot" null null))
  (set `self.GeneratedTile` _returnvalue)
  (goto _label))

(event `SpawnStart`
  (params (Row :type Integer) (Column :type Integer))
  (bind _transform (`self.CoordsToTransform` Row Column))
  (bind _returnvalue (`|SpawnActorFromClass` "/Game/Tile_Start.Tile_Start_C" _transform "Undefined" "MultiplyWithRoot" null null))
  (set `self.GeneratedTile` _returnvalue)
  (goto _label))

(event `Add To Actor Array`
  (bind _output_0 (break `/Game/TileActorRow` (`|GetArrayItem` (`self.Tile Actors`) (`self.Row Index`))))
  (bind _output_get (set `self.Tile Actor Row` _output_0))
  (`KismetArrayLibrary.Array_Set` _output_get (`self.Column Index`) (`self.GeneratedTile`) true)
  (`KismetArrayLibrary.Array_Set` (`self.Tile Actors`) (`self.Row Index`) (make `/Game/TileActorRow` (`self.Tile Actor Row`))))

(event `GenerateLevel`
  (bind _outrownames (`DataTableFunctionLibrary.GetDataTableRowNames` "/Game/Level1Layout.Level1Layout"))
  (for (_array_element _array_index) _outrownames
    (set `self.Row Index` _array_index)
    (bind _returnvalue (`|GetDataTableRow` "/Game/Level1Layout.Level1Layout" _array_element)
      (:`then`
        (for (_array_element_2 _array_index_2) (`|MakeArray` (break `/Game/TileRow` _returnvalue) (`.Col2_15_671E648E4C647793CEC580BF4E15FD69` (break `/Game/TileRow` _returnvalue)) (`.Col3_16_1BA4002149BDDAED163BE7961001554A` (break `/Game/TileRow` _returnvalue)) (`.Col4_17_8B636DBE4F792236D1730E99BD66B86E` (break `/Game/TileRow` _returnvalue)) (`.Col5_18_29F5ED6B42917F1E54C62A90B1DD1943` (break `/Game/TileRow` _returnvalue)) (`.Col6_19_B119384E406B3C962BB531AB3E0F2B94` (break `/Game/TileRow` _returnvalue)) (`.Col7_20_A4F3F7234459432FA5B9D594AAA6F801` (break `/Game/TileRow` _returnvalue)) (`.Col8_21_04C638DC437976CED9EAF0A7CCE4041A` (break `/Game/TileRow` _returnvalue)) (`.Col9_22_558CC10F480992C2371990965A1104F3` (break `/Game/TileRow` _returnvalue)) (`.Col10_23_6F56153344F7AFE2526CFDB91DF362A7` (break `/Game/TileRow` _returnvalue)) (`.Col11_24_1024AE0147287A4AB3F3168EC6E52E99` (break `/Game/TileRow` _returnvalue)) (`.Col12_25_BE46EA474373C37617FD2AA764196F65` (break `/Game/TileRow` _returnvalue)) (`.Col13_26_F03605AF4EB610AE9E3AF98A311F01B1` (break `/Game/TileRow` _returnvalue)) (`.Col14_28_C31EFEC2497B5E15B4E9C1A0BF15EF93` (break `/Game/TileRow` _returnvalue)) (`.Col15_30_E5297D6044193CEAE3C24DBA2E66967B` (break `/Game/TileRow` _returnvalue)) (`.Col16_32_EC0F68DA4B6A4A9DC0506ABD2A972606` (break `/Game/TileRow` _returnvalue)))
          (set `self.Column Index` _array_index_2)
          (switch `/Game/TileTypes` _array_element_2
            (:`NewEnumerator0`
              (`self.SpawnEmpty` (`self.Row Index`) (`self.Column Index`)))
            (:`NewEnumerator2`
              (`self.SpawnStart` (`self.Row Index`) (`self.Column Index`)))
            (:`NewEnumerator3`
              (`self.SpawnBasic` (`self.Row Index`) (`self.Column Index`))))
          (`self.Add To Actor Array`))))))

(event `ClearLevel`
  (bind _outactors (`GameplayStatics.GetAllActorsOfClass` "/Game/Tile.Tile_C"))
  (for _array_element _outactors
    (`self.K2_DestroyActor` _array_element)))

(fn `CoordsToTransform`
  (params (Row :type Integer) (Column :type Integer))
  (returns (Transform :type "Transform Structure"))
  (return (`KismetMathLibrary.MakeTransform` (`KismetMathLibrary.MakeVector` (`KismetMathLibrary.Conv_IntToDouble` (+ (* Row -100) 50)) (`KismetMathLibrary.Conv_IntToDouble` (+ (* Column 100) 50))))))

(fn `UserConstructionScript`)