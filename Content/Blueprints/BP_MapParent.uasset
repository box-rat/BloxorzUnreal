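; BP_MapParent builds a tile-based puzzle level from a data table and handles level-wide tile reactions.
; GenerateLevel takes row names from the DataTable variable but reads rows from hardcoded Level7Layout, mapping sixteen column values to typed tile spawns.
; Spawners convert grid indices to world transforms and stamp coordinates, then AddToActorArray stores each tile in a nested row-struct array.
; Fail, complete and clear events act on every Tile actor, the first two after a delay.
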(event `SpawnFlip`
  (params (Row :type Integer) (Column :type Integer))
  (bind _transform (`self.CoordsToTransform` Row Column))
  (bind _returnvalue (`|SpawnActorFromClass` "/Game/Tiles/Tile_Flip.Tile_Flip_C" _transform "Undefined" "MultiplyWithRoot" null null))
  (set `self.GeneratedTile` _returnvalue)
  (bind _output_get (set `/Game/Tiles/Tile.Coordinates` (`KismetMathLibrary.MakeVector2D` (`KismetMathLibrary.Conv_IntToDouble` (`self.Column Index`)) (`KismetMathLibrary.Conv_IntToDouble` (`self.Row Index`))) (`self.GeneratedTile`) :!label _label))
  (`KismetSystemLibrary.LogString` (`KismetStringLibrary.Concat_StrStr` (`KismetStringLibrary.Conv_Vector2dToString` _output_get) " :: " (`KismetSystemLibrary.GetDisplayName` (`self.GeneratedTile`)))))

(event `SpawnOrange`
  (params (Row :type Integer) (Column :type Integer))
  (bind _transform (`self.CoordsToTransform` Row Column))
  (bind _returnvalue (`|SpawnActorFromClass` "/Game/Tiles/Tile_Orange.Tile_Orange_C" _transform "Undefined" "MultiplyWithRoot" null null))
  (set `self.GeneratedTile` _returnvalue)
  (goto _label))

(event `SpawnExitTile`
  (params (Row :type Integer) (Column :type Integer))
  (bind _transform (`self.CoordsToTransform` Row Column))
  (bind _returnvalue (`|SpawnActorFromClass` "/Game/Tiles/Tile_Exit.Tile_Exit_C" _transform "Undefined" "MultiplyWithRoot" null null))
  (set `self.GeneratedTile` _returnvalue)
  (goto _label))

(event `SpawnOButton`
  (params (Row :type Integer) (Column :type Integer))
  (bind _transform (`self.CoordsToTransform` Row Column))
  (bind _returnvalue (`|SpawnActorFromClass` "/Game/Tiles/Tile_OButton.Tile_OButton_C" _transform "Undefined" "MultiplyWithRoot" null null))
  (set `self.GeneratedTile` _returnvalue)
  (goto _label))

(event `SpawnXButton`
  (params (Row :type Integer) (Column :type Integer))
  (bind _transform (`self.CoordsToTransform` Row Column))
  (bind _returnvalue (`|SpawnActorFromClass` "/Game/Tiles/Tile_XButton.Tile_XButton_C" _transform "Undefined" "MultiplyWithRoot" null null))
  (set `self.GeneratedTile` _returnvalue)
  (goto _label))

(event `SpawnEmpty`
  (params (Row :type Integer) (Column :type Integer))
  (bind _transform (`self.CoordsToTransform` Row Column))
  (bind _returnvalue (`|SpawnActorFromClass` "/Game/Tiles/Tile_Empty.Tile_Empty_C" _transform "Undefined" "MultiplyWithRoot" null null))
  (set `self.GeneratedTile` _returnvalue)
  (goto _label))

(event `SpawnBasic`
  (params (Row :type Integer) (Column :type Integer))
  (bind _transform (`self.CoordsToTransform` Row Column))
  (bind _returnvalue (`|SpawnActorFromClass` "/Game/Tiles/Tile_Basic.Tile_Basic_C" _transform "Undefined" "MultiplyWithRoot" null null))
  (set `self.GeneratedTile` _returnvalue)
  (goto _label))

(event `SpawnStart`
  (params (Row :type Integer) (Column :type Integer))
  (bind _transform (`self.CoordsToTransform` Row Column))
  (bind _returnvalue (`|SpawnActorFromClass` "/Game/Tiles/Tile_Start.Tile_Start_C" _transform "Undefined" "MultiplyWithRoot" null null))
  (set `self.GeneratedTile` _returnvalue)
  (goto _label))

(event `Add To Actor Array`
  (bind _output_0 (break `/Game/Data/TileActorRow` (`|GetArrayItem` (`self.Tile Actors`) (`self.Row Index`))))
  (bind _output_get (set `self.Tile Actor Row` _output_0))
  (`KismetArrayLibrary.Array_Set` _output_get (`self.Column Index`) (`self.GeneratedTile`) true)
  (`KismetArrayLibrary.Array_Set` (`self.Tile Actors`) (`self.Row Index`) (make `/Game/Data/TileActorRow` (`self.Tile Actor Row`))))

(event `GenerateLevel`
  (bind _outrownames (`DataTableFunctionLibrary.GetDataTableRowNames` (`self.DataTable`)))
  (for (_array_element _array_index) _outrownames
    (set `self.Row Index` _array_index)
    (bind _returnvalue (`|GetDataTableRow` "/Game/LevelLayouts/Level7Layout.Level7Layout" _array_element)
      (:`then`
        (for (_array_element_2 _array_index_2) (`|MakeArray` (break `/Game/Data/TileRow` _returnvalue) (`.Col2_15_671E648E4C647793CEC580BF4E15FD69` (break `/Game/Data/TileRow` _returnvalue)) (`.Col3_16_1BA4002149BDDAED163BE7961001554A` (break `/Game/Data/TileRow` _returnvalue)) (`.Col4_17_8B636DBE4F792236D1730E99BD66B86E` (break `/Game/Data/TileRow` _returnvalue)) (`.Col5_18_29F5ED6B42917F1E54C62A90B1DD1943` (break `/Game/Data/TileRow` _returnvalue)) (`.Col6_19_B119384E406B3C962BB531AB3E0F2B94` (break `/Game/Data/TileRow` _returnvalue)) (`.Col7_20_A4F3F7234459432FA5B9D594AAA6F801` (break `/Game/Data/TileRow` _returnvalue)) (`.Col8_21_04C638DC437976CED9EAF0A7CCE4041A` (break `/Game/Data/TileRow` _returnvalue)) (`.Col9_22_558CC10F480992C2371990965A1104F3` (break `/Game/Data/TileRow` _returnvalue)) (`.Col10_23_6F56153344F7AFE2526CFDB91DF362A7` (break `/Game/Data/TileRow` _returnvalue)) (`.Col11_24_1024AE0147287A4AB3F3168EC6E52E99` (break `/Game/Data/TileRow` _returnvalue)) (`.Col12_25_BE46EA474373C37617FD2AA764196F65` (break `/Game/Data/TileRow` _returnvalue)) (`.Col13_26_F03605AF4EB610AE9E3AF98A311F01B1` (break `/Game/Data/TileRow` _returnvalue)) (`.Col14_28_C31EFEC2497B5E15B4E9C1A0BF15EF93` (break `/Game/Data/TileRow` _returnvalue)) (`.Col15_30_E5297D6044193CEAE3C24DBA2E66967B` (break `/Game/Data/TileRow` _returnvalue)) (`.Col16_32_EC0F68DA4B6A4A9DC0506ABD2A972606` (break `/Game/Data/TileRow` _returnvalue)))
          (set `self.Column Index` _array_index_2)
          (switch `/Game/Data/TileTypes` _array_element_2
            (:`NewEnumerator0`
              (`self.SpawnEmpty` (`self.Row Index`) (`self.Column Index`)))
            (:`NewEnumerator1`
              (`self.SpawnExitTile` (`self.Row Index`) (`self.Column Index`)))
            (:`NewEnumerator2`
              (`self.SpawnStart` (`self.Row Index`) (`self.Column Index`)))
            (:`NewEnumerator3`
              (`self.SpawnBasic` (`self.Row Index`) (`self.Column Index`)))
            (:`NewEnumerator4`
              (`self.SpawnOrange` (`self.Row Index`) (`self.Column Index`)))
            (:`NewEnumerator5`
              (`self.SpawnFlip` (`self.Row Index`) (`self.Column Index`)))
            (:`NewEnumerator6`
              (`self.SpawnOButton` (`self.Row Index`) (`self.Column Index`)))
            (:`NewEnumerator7`
              (`self.SpawnXButton` (`self.Row Index`) (`self.Column Index`))))
          (`self.Add To Actor Array`))))))

(event `FailLevel`
  (`KismetSystemLibrary.PrintString` "FailLevel")
  (`KismetSystemLibrary.Delay` 0.5)
  (bind _outactors (`GameplayStatics.GetAllActorsOfClass` "/Game/Tiles/Tile.Tile_C"))
  (for _array_element _outactors
    (`/Game/Tiles/Tile.Fail` _array_element)))

(event `CompleteLevel`
  (`KismetSystemLibrary.PrintString` "CompleteLevel")
  (`KismetSystemLibrary.Delay` 0.5)
  (bind _outactors (`GameplayStatics.GetAllActorsOfClass` "/Game/Tiles/Tile.Tile_C"))
  (for _array_element _outactors
    (`/Game/Tiles/Tile.VictorySpin` _array_element)))

(event `ClearLevel`
  (bind _outactors (`GameplayStatics.GetAllActorsOfClass` "/Game/Tiles/Tile.Tile_C"))
  (for _array_element _outactors
    (`self.K2_DestroyActor` _array_element)))

(fn `CoordsToTransform`
  (params (Row :type Integer) (Column :type Integer))
  (returns (Transform :type "Transform Structure"))
  (return (`KismetMathLibrary.MakeTransform` (`KismetMathLibrary.MakeVector` (`KismetMathLibrary.Conv_IntToDouble` (+ (* Row -100) 50)) (`KismetMathLibrary.Conv_IntToDouble` (+ (* Column 100) 50))))))

(fn `UserConstructionScript`)