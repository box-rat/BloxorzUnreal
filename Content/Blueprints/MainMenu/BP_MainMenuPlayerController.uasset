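; Main menu player controller that sets up the menu scene, music and UI.
; BeginPlay starts the theme, switches to UI-only input with a cursor, views through BP_Camera, layers the oscillate, menu and black screen widgets, then fades in from black.
; FadeToBlack and FadeFromBlack drive black screen opacity with timelines.
; ObscureLogo reverses a timeline to animate the title's text and outline alpha.
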(event `self.ReceiveBeginPlay`
  (`FMODBlueprintStatics.PlayEvent2D` "/Game/FMOD/Events/MainTheme.MainTheme")
  (bind _returnvalue (`|CreateWidget` "/Game/UI/WBP_BlackOscillate.WBP_BlackOscillate_C"))
  (`UserWidget.AddToViewport` _returnvalue 0)
  (`WidgetBlueprintLibrary.SetInputMode_UIOnlyEx` self null)
  (set `self.bShowMouseCursor` true)
  (bind _returnvalue_2 (`GameplayStatics.GetActorOfClass` "/Game/Blueprints/BP_Camera.BP_Camera_C"))
  (`self.SetViewTargetWithBlend` _returnvalue_2)
  (bind _returnvalue_3 (`|CreateWidget` "/Game/UI/WBP_MainMenu.WBP_MainMenu_C"))
  (set `self.MainMenu` _returnvalue_3)
  (`UserWidget.AddToViewport` _returnvalue_3 1)
  (bind _returnvalue_4 (`|CreateWidget` "/Game/UI/WBP_BlackScreen.WBP_BlackScreen_C"))
  (set `self.BlackScreen` _returnvalue_4)
  (`UserWidget.AddToViewport` _returnvalue_4 100)
  (`self.FadeFromBlack`))

(event `FadeToBlack`
  (bind (_direction _newtrack_0) (`Timeline|Fader` :!via `PlayFromStart`)
    (:`Update`
      (`Image.SetOpacity` (`/Game/UI/WBP_BlackScreen.Black` (`self.BlackScreen`)) _newtrack_0))))

(event `ObscureLogo`
  (bind _title (`/Game/UI/WBP_MainMenu.Title` (`self.MainMenu`)))
  (bind _font (`TextBlock.Font` _title))
  (bind _colorandopacity (`TextBlock.ColorAndOpacity` _title))
  (bind (_direction _newtrack_0) (`Timeline|Obscure` :!via `ReverseFromEnd`)
    (:`Update`
      (`TextBlock.SetFont` _title (make `SlateFontInfo` (break `SlateFontInfo` _font) (`.FontMaterial` (break `SlateFontInfo` _font)) (make `FontOutlineSettings` (break `FontOutlineSettings` (`.OutlineSettings` (break `SlateFontInfo` _font))) (`.bMiteredCorners` (break `FontOutlineSettings` (`.OutlineSettings` (break `SlateFontInfo` _font)))) (`.bSeparateFillAlpha` (break `FontOutlineSettings` (`.OutlineSettings` (break `SlateFontInfo` _font)))) (`.bApplyOutlineToDropShadows` (break `FontOutlineSettings` (`.OutlineSettings` (break `SlateFontInfo` _font)))) (`.OutlineMaterial` (break `FontOutlineSettings` (`.OutlineSettings` (break `SlateFontInfo` _font)))) (make `LinearColor` (break `LinearColor` (`.OutlineColor` (break `FontOutlineSettings` (`.OutlineSettings` (break `SlateFontInfo` _font))))) (`.G` (break `LinearColor` (`.OutlineColor` (break `FontOutlineSettings` (`.OutlineSettings` (break `SlateFontInfo` _font)))))) (`.B` (break `LinearColor` (`.OutlineColor` (break `FontOutlineSettings` (`.OutlineSettings` (break `SlateFontInfo` _font)))))) (`KismetMathLibrary.Lerp` 0.0 0.733333 _newtrack_0))) (`.TypefaceFontName` (break `SlateFontInfo` _font)) (`.Size` (break `SlateFontInfo` _font)) (`.LetterSpacing` (break `SlateFontInfo` _font)) (`.SkewAmount` (break `SlateFontInfo` _font)) (`.bForceMonospaced` (break `SlateFontInfo` _font)) (`.MonospacedWidth` (break `SlateFontInfo` _font))))
      (`TextBlock.SetColorAndOpacity` _title (make `SlateColor` (make `LinearColor` (break `LinearColor` (break `SlateColor` _colorandopacity)) (`.G` (break `LinearColor` (break `SlateColor` _colorandopacity))) (`.B` (break `LinearColor` (break `SlateColor` _colorandopacity))) _newtrack_0) (`.ColorUseRule` (break `SlateColor` _colorandopacity)))))))

(event `FadeFromBlack`
  (bind (_direction _newtrack_0) (`Timeline|Other Fader` :!via `ReverseFromEnd`)
    (:`Update`
      (`Image.SetOpacity` (`/Game/UI/WBP_BlackScreen.Black` (`self.BlackScreen`)) _newtrack_0))))

(fn `UserConstructionScript`)