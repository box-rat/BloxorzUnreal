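; Main menu pawn that handles starting a new save or loading the existing one in a single save slot.
; On BeginPlay it caches the BP_GameInstance.
; CreateNewSave wipes the slot and writes a fresh BP_SaveGame, while LoadSave reads the stored one.
; Both copy moves, attempts, level and the save object into the game instance, but only LoadSave also copies the timer.
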(event `self.ReceiveBeginPlay`
  (bind _asbp_game_instance (cast `/Game/Blueprints/BP_GameInstance` (`GameplayStatics.GetGameInstance`)))
  (set `self.Instance` _asbp_game_instance))

(event `CreateNewSave`
  (`GameplayStatics.DeleteGameInSlot` "Slot1")
  (bind _returnvalue (`GameplayStatics.CreateSaveGameObject` "/Game/Blueprints/BP_SaveGame.BP_SaveGame_C"))
  (set `self.SaveGame` _returnvalue)
  (bind _returnvalue_2 (`GameplayStatics.SaveGameToSlot` (`self.SaveGame`) "Slot1"))
  (if _returnvalue_2
    (set `/Game/Blueprints/BP_GameInstance.MovesAtStart` (`/Game/Blueprints/BP_SaveGame.Moves` (`self.SaveGame`)) (`self.Instance`))
    (set `/Game/Blueprints/BP_GameInstance.Attempts` (`/Game/Blueprints/BP_SaveGame.Attempts` (`self.SaveGame`)) (`self.Instance`))
    (set `/Game/Blueprints/BP_GameInstance.Level` (`/Game/Blueprints/BP_SaveGame.Level` (`self.SaveGame`)) (`self.Instance`))
    (set `/Game/Blueprints/BP_GameInstance.SaveGame` (`self.SaveGame`) (`self.Instance`))
    (else
      (`KismetSystemLibrary.PrintString` "Failed to save!"))))

(event `LoadSave`
  (bind _returnvalue (`GameplayStatics.LoadGameFromSlot` "Slot1"))
  (bind _asbp_save_game (cast `/Game/Blueprints/BP_SaveGame` _returnvalue)
    (:`then`
      (set `self.SaveGame` _asbp_save_game)
      (set `/Game/Blueprints/BP_GameInstance.MovesAtStart` (`/Game/Blueprints/BP_SaveGame.Moves` (`self.SaveGame`)) (`self.Instance`))
      (set `/Game/Blueprints/BP_GameInstance.Attempts` (`/Game/Blueprints/BP_SaveGame.Attempts` (`self.SaveGame`)) (`self.Instance`))
      (set `/Game/Blueprints/BP_GameInstance.Level` (`/Game/Blueprints/BP_SaveGame.Level` (`self.SaveGame`)) (`self.Instance`))
      (set `/Game/Blueprints/BP_GameInstance.Timer` (`/Game/Blueprints/BP_SaveGame.Timer` (`self.SaveGame`)) (`self.Instance`))
      (set `/Game/Blueprints/BP_GameInstance.SaveGame` (`self.SaveGame`) (`self.Instance`)))
    (:`CastFailed`
      (`KismetSystemLibrary.PrintString` "Cast to BP_SaveGame failed somehow?"))))

(fn `UserConstructionScript`)