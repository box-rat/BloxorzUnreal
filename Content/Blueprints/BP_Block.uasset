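; Player-controlled two-cell block for a Bloxorz-style tile puzzle that drops in at the start tile and rolls with WASD.
; Each roll moves a pivot to the block's edge, updates both grid coordinates and pre-checks tiles.
; When the animation ends, it fires buttons, clears the level or fails it with a physics fall, shifting center of mass toward any unsupported end.
; Input during a roll snaps it to completion before starting the next.
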(event `Rotate`
  (params (`Block Orientation` :type "/Game/Data/E_BlockOrientation Enum" :default "NewEnumerator0") (`Input Direction` :type "/Game/Data/E_Directions Enum" :default "NewEnumerator0"))
  (bind (_relativerotation_roll _relativerotation_pitch _relativerotation_yaw) (`KismetMathLibrary.BreakRotator` (`SceneComponent.RelativeRotation` (`self.Pivot`))))
  (bind (_relativerotation_roll_2 _relativerotation_pitch_2 _relativerotation_yaw_2) (`KismetMathLibrary.BreakRotator` (`SceneComponent.RelativeRotation` (`self.Pivot`))))
  (bind (_relativerotation_roll_3 _relativerotation_pitch_3 _relativerotation_yaw_3) (`KismetMathLibrary.BreakRotator` (`SceneComponent.RelativeRotation` (`self.Pivot`))))
  (bind (_relativerotation_roll_4 _relativerotation_pitch_4 _relativerotation_yaw_4) (`KismetMathLibrary.BreakRotator` (`SceneComponent.RelativeRotation` (`self.Pivot`))))
  (if (`self.RotateEnabled`)
    (if (`self.Rotating?`)
      (`self.BufferedInput` `Block Orientation` `Input Direction`)
      (else
        (set `self.Rotating?` true)
        (`self.Set Pivot` `Block Orientation` `Input Direction`)
        (`self.setNewCoordinates` `Block Orientation` `Input Direction`)
        (`self.CheckTriggers`)
        (`SceneComponent.K2_AttachToComponent` (`self.Block`) (`self.Pivot`) "None" "KeepWorld" "KeepRelative" "KeepRelative" false)
        (switch `/Game/Data/E_Directions` `Input Direction`
          (:`NewEnumerator0`
            (set `self.EndRot` (`KismetMathLibrary.MakeRotator` _relativerotation_roll_2 (+ _relativerotation_pitch_2 -90.0) _relativerotation_yaw_2))
            (bind (_direction _timeline_alpha) (`Timeline|Timeline` :`NewTime` 0.25 :!via `PlayFromStart` :!label _label)
              (:`Update`
                (`SceneComponent.K2_SetRelativeRotation` (`self.Pivot`) (`KismetMathLibrary.RLerp` (struct) (`self.EndRot`) _timeline_alpha true) false false))
              (:`Finished`
                (`self.ResetBlock`)
                (`self.ExecuteTriggers`))))
          (:`NewEnumerator1`
            (set `self.EndRot` (`KismetMathLibrary.MakeRotator` _relativerotation_roll_3 (+ _relativerotation_pitch_3 90.0) _relativerotation_yaw_3))
            (goto _label :!via `PlayFromStart`))
          (:`NewEnumerator2`
            (set `self.EndRot` (`KismetMathLibrary.MakeRotator` (+ _relativerotation_roll_4 -90.0) _relativerotation_pitch_4 _relativerotation_yaw_4))
            (goto _label :!via `PlayFromStart`))
          (:`NewEnumerator3`
            (set `self.EndRot` (`KismetMathLibrary.MakeRotator` (+ _relativerotation_roll 90.0) _relativerotation_pitch _relativerotation_yaw))
            (goto _label :!via `PlayFromStart`)))))))

(event `Stop Timeline`
  (goto _label :!via `Stop`))

(event `BufferedInput`
  (params (`Block Orientation` :type "/Game/Data/E_BlockOrientation Enum" :default "NewEnumerator0") (`Input Direction` :type "/Game/Data/E_Directions Enum" :default "NewEnumerator0"))
  (`self.Stop Timeline`)
  (`SceneComponent.K2_SetRelativeRotation` (`self.Pivot`) (`self.EndRot`) false false)
  (`self.ResetBlock`)
  (`self.ExecuteTriggers`)
  (`self.Rotate` `Block Orientation` `Input Direction`))

(event `Set Pivot`
  (params (`Block Orientation` :type "/Game/Data/E_BlockOrientation Enum" :default "NewEnumerator0") (`Input Direction` :type "/Game/Data/E_Directions Enum" :default "NewEnumerator0"))
  (switch `/Game/Data/E_Directions` `Input Direction`
    (:`NewEnumerator0`
      (switch `/Game/Data/E_BlockOrientation` `Block Orientation`
        (:`NewEnumerator0`
          (set `self.PivotPoint` (100.0 0.0 -50.0))
          (set `self.BlockOrientation` "NewEnumerator2"))
        (:`NewEnumerator1`
          (set `self.PivotPoint` (50.0 0.0 -50.0))
          (set `self.BlockOrientation` "NewEnumerator1"))
        (:`NewEnumerator2`
          (set `self.PivotPoint` (50.0 0.0 -100.0))
          (set `self.BlockOrientation` "NewEnumerator0"))))
    (:`NewEnumerator1`
      (switch `/Game/Data/E_BlockOrientation` `Block Orientation`
        (:`NewEnumerator0`
          (set `self.PivotPoint` (-100.0 0.0 -50.0))
          (set `self.BlockOrientation` "NewEnumerator2"))
        (:`NewEnumerator1`
          (set `self.PivotPoint` (-50.0 0.0 -50.0))
          (set `self.BlockOrientation` "NewEnumerator1"))
        (:`NewEnumerator2`
          (set `self.PivotPoint` (-50.0 0.0 -100.0))
          (set `self.BlockOrientation` "NewEnumerator0"))))
    (:`NewEnumerator2`
      (switch `/Game/Data/E_BlockOrientation` `Block Orientation`
        (:`NewEnumerator0`
          (set `self.PivotPoint` (0.0 -50.0 -50.0))
          (set `self.BlockOrientation` "NewEnumerator0"))
        (:`NewEnumerator1`
          (set `self.PivotPoint` (0.0 -100.0 -50.0))
          (set `self.BlockOrientation` "NewEnumerator2"))
        (:`NewEnumerator2`
          (set `self.PivotPoint` (0.0 -50.0 -100.0))
          (set `self.BlockOrientation` "NewEnumerator1"))))
    (:`NewEnumerator3`
      (switch `/Game/Data/E_BlockOrientation` `Block Orientation`
        (:`NewEnumerator0`
          (set `self.PivotPoint` (0.0 50.0 -50.0))
          (set `self.BlockOrientation` "NewEnumerator0"))
        (:`NewEnumerator1`
          (set `self.PivotPoint` (0.0 100.0 -50.0))
          (set `self.BlockOrientation` "NewEnumerator2"))
        (:`NewEnumerator2`
          (set `self.PivotPoint` (0.0 50.0 -100.0))
          (set `self.BlockOrientation` "NewEnumerator1")))))
  (`SceneComponent.K2_SetRelativeLocation` (`self.Pivot`) (`self.PivotPoint`) false false))

(event `Initialize`
  (bind _returnvalue (`GameplayStatics.GetActorOfClass` "/Game/Blueprints/BP_Camera.BP_Camera_C"))
  (`PlayerController.SetViewTargetWithBlend` (`GameplayStatics.GetPlayerController` 0) _returnvalue 0.0 "VTBlend_Linear" 0.0 false)
  (bind _returnvalue_2 (`GameplayStatics.GetActorOfClass` "/Game/Blueprints/BP_MapParent.BP_MapParent_C"))
  (set `self.MapParent` _returnvalue_2)
  (bind _returnvalue_3 (`GameplayStatics.GetActorOfClass` "/Game/Tiles/Tile_Start.Tile_Start_C"))
  (bind (_returnvalue_x _returnvalue_y _returnvalue_z) (`KismetMathLibrary.BreakVector` (`self.K2_GetActorLocation` _returnvalue_3)))
  (`self.K2_SetActorLocation` (`KismetMathLibrary.MakeVector` _returnvalue_x _returnvalue_y (+ _returnvalue_z 50.0)))
  (bind _coordinates (`/Game/Tiles/Tile.Coordinates` _returnvalue_3))
  (set `self.TopCoord` _coordinates)
  (set `self.BottomCoord` _coordinates)
  (`self.BlockIntro`))

(event `self.ReceiveBeginPlay`
  (`self.Initialize`))

(event `self.ReceiveTick`
  (params (DeltaSeconds :type "Float (single-precision)")))

(event `Key|W`
  (params (Key :type "Key Structure"))
  (:`Pressed`
    (`self.Rotate` (`self.BlockOrientation`))))

(event `Key|D`
  (params (Key :type "Key Structure"))
  (:`Pressed`
    (`self.Rotate` (`self.BlockOrientation`) "NewEnumerator3")))

(event `Key|A`
  (params (Key :type "Key Structure"))
  (:`Pressed`
    (`self.Rotate` (`self.BlockOrientation`) "NewEnumerator2")))

(event `Key|S`
  (params (Key :type "Key Structure"))
  (:`Pressed`
    (`self.Rotate` (`self.BlockOrientation`) "NewEnumerator1")))

(event `BlockIntro`
  (bind (_returnvalue_x _returnvalue_y) (`KismetMathLibrary.BreakVector` (`SceneComponent.K2_GetComponentLocation` (`self.Block`))))
  (bind (_returnvalue_x_2 _returnvalue_y_2) (`KismetMathLibrary.BreakVector` (`SceneComponent.K2_GetComponentLocation` (`self.Block`))))
  (`GameplayStatics.SetGlobalTimeDilation` 1.0)
  (`SceneComponent.K2_SetWorldLocation` (`self.Block`) (`KismetMathLibrary.MakeVector` _returnvalue_x _returnvalue_y 1500.0) false false)
  (`KismetSystemLibrary.Delay` 1.1)
  (bind (_direction _newtrack_0) (`Timeline|Timeline_0`)
    (:`Update`
      (`SceneComponent.K2_SetWorldLocation` (`self.Block`) (`KismetMathLibrary.MakeVector` _returnvalue_x_2 _returnvalue_y_2 (`KismetMathLibrary.Lerp` 1000.0 100.0 _newtrack_0)) false false))
    (:`Finished`
      (bind (_direction_2 _newtrack_0_2) (`Timeline|Timeline_1` :!via `PlayFromStart`)
        (:`Update`
          (bind _returnvalue (`KismetMathLibrary.Lerp` 0.0 1.0 _newtrack_0_2))
          (`SceneComponent.K2_SetWorldRotation` (`self.Block`) (`KismetMathLibrary.MakeRotator` _returnvalue _returnvalue) false false))
        (:`Finished`
          (set `self.RotateEnabled` true)
          (`self.ResetBlock`))))))

(event `CheckTriggers`
  (`self.getTileActors` (`self.TopCoord`) (`self.BottomCoord`))
  (`|ExecutionSequence`
    (:`then_0`
      (bind _output (`self.exit?`))
      (bind _output_get (set `self.shouldExit?` _output))
      (if _output_get
        (set `self.RotateEnabled` false)))
    (:`then_1`
      (bind (_result _illegalblock) (`self.isLegal?`))
      (bind _output_get_2 (set `self.IllegalMoveMade?` (not _result)))
      (if _output_get_2
        (set `self.RotateEnabled` false)
        (set `self.IllegalBlock` _illegalblock)))
    (:`then_2`
      (cast `/Game/Tiles/Tile_OButton` (`self.TopTile`))
      (set `self.FireTopTileOButton?` true))
    (:`then_3`
      (if (`|EnumInequality` (`self.BlockOrientation`) "NewEnumerator2")
        (cast `/Game/Tiles/Tile_OButton` (`self.BottomTile`))
        (set `self.FireBottomOTileButton?` true)))
    (:`then_4`
      (cast `/Game/Tiles/Tile_XButton` (`self.TopTile`))
      (if (`|EnumEquality` (`self.BlockOrientation`) "NewEnumerator2")
        (set `self.FireXButton?` true)))
    (:`then_5`
      (if (`|EnumEquality` (`self.BlockOrientation`) "NewEnumerator2")
        (cast `/Game/Tiles/Tile_Orange` (`self.TopTile`))
        (set `self.IllegalBlock` "Both")
        (set `self.RotateEnabled` false)
        (set `self.IllegalMoveMade?` true)
        (set `self.OrangeTileTriggered?` true)))))

(event `ExecuteTriggers`
  (`|ExecutionSequence`
    (:`then_0`
      (if (`self.IllegalMoveMade?`)
        (`self.IllegalMove`)
        (`/Game/Blueprints/BP_MapParent.FailLevel` (`self.MapParent`))))
    (:`then_1`
      (if (`self.shouldExit?`)
        (`self.Level Clear`)))
    (:`then_2`
      (if (`self.FireTopTileOButton?`)
        (bind _astile_obutton (cast `/Game/Tiles/Tile_OButton` (`self.TopTile`)))
        (`/Game/Tiles/Tile_OButton.Fire` _astile_obutton)
        (set `self.FireTopTileOButton?` false)))
    (:`then_3`
      (if (`self.FireBottomOTileButton?`)
        (bind _astile_obutton_2 (cast `/Game/Tiles/Tile_OButton` (`self.BottomTile`)))
        (`/Game/Tiles/Tile_OButton.Fire` _astile_obutton_2)
        (set `self.FireBottomOTileButton?` false)))
    (:`then_4`
      (if (`self.FireXButton?`)
        (bind _astile_xbutton (cast `/Game/Tiles/Tile_XButton` (`self.TopTile`)))
        (`/Game/Tiles/Tile_XButton.Fire` _astile_xbutton)
        (set `self.FireXButton?` false)))
    (:`then_5`
      (if (`self.OrangeTileTriggered?`)
        (bind _astile_orange (cast `/Game/Tiles/Tile_Orange` (`self.TopTile`)))
        (`/Game/Tiles/Tile_Orange.Fall` _astile_orange)))))

(event `Level Clear`
  (bind _block (`self.Block`))
  (set `self.RotateEnabled` false)
  (`PrimitiveComponent.SetSimulatePhysics` _block true)
  (`PrimitiveComponent.SetCollisionEnabled` _block "QueryOnly")
  (`PrimitiveComponent.SetMaterial` (`self.Block`) 0 "/Game/Materials/BlockMat1.BlockMat1"))

(fn `exit?`
  (returns (Output :type Boolean))
  (cast `/Game/Tiles/Tile_Exit` (`self.TopTile`)
    (:`then`
      (return (`|EnumEquality` (`self.BlockOrientation`) "NewEnumerator2")))
    (:`CastFailed`
      (return false))))

(fn `getTileActors`
  (params (`Top Coord` :type "Vector2D Structure") (`Bottom Coord` :type "Vector2D Structure"))
  (bind _output_0 (break `/Game/Data/TileActorRow` (`|GetArrayItem` (`/Game/Blueprints/BP_MapParent.Tile Actors` (`self.MapParent`)) (`KismetMathLibrary.FTrunc` `Bottom Coord_Y`))))
  (bind _output_0_2 (break `/Game/Data/TileActorRow` (`|GetArrayItem` (`/Game/Blueprints/BP_MapParent.Tile Actors` (`self.MapParent`)) (`KismetMathLibrary.FTrunc` `Top Coord_Y`))))
  (set `self.TopTile` (`|GetArrayItem` _output_0_2 (`KismetMathLibrary.FTrunc` `Top Coord_X`)))
  (set `self.BottomTile` (`|GetArrayItem` _output_0 (`KismetMathLibrary.FTrunc` `Bottom Coord_X`))))

(fn `IllegalMove`
  (bind _block (`self.Block`))
  (bind _block_2 (`self.Block`))
  (bind (_bottomcoord_x _bottomcoord_y) (`KismetMathLibrary.BreakVector2D` (`self.BottomCoord`)))
  (bind _block_3 (`self.Block`))
  (bind (_topcoord_x _topcoord_y) (`KismetMathLibrary.BreakVector2D` (`self.TopCoord`)))
  (bind (_returnvalue_x _returnvalue_y) (`KismetMathLibrary.BreakVector` (`SceneComponent.K2_GetComponentLocation` (`self.Block`))))
  (bind (_returnvalue_x_2 _returnvalue_y_2) (`KismetMathLibrary.BreakVector` (`SceneComponent.K2_GetComponentLocation` (`self.Block`))))
  (switch `string` (`self.IllegalBlock`)
    (:`Top`
      (bind _transform (`/Game/Blueprints/BP_MapParent.CoordsToTransform` (`self.MapParent`) (`KismetMathLibrary.FTrunc` _topcoord_y) (`KismetMathLibrary.FTrunc` _topcoord_x)))
      (`PrimitiveComponent.SetCenterOfMass` (`self.Block`) (* (`KismetMathLibrary.InverseTransformDirection` (`SceneComponent.K2_GetComponentToWorld` (`self.Block`)) (`KismetMathLibrary.Normal` (- (.location _transform) (`KismetMathLibrary.MakeVector` _returnvalue_x _returnvalue_y)))) 50) "None")
      (`PrimitiveComponent.SetSimulatePhysics` _block_3 true)
      (`PrimitiveComponent.SetCollisionEnabled` _block_3 "QueryAndPhysics"))
    (:`Bottom`
      (bind _transform_2 (`/Game/Blueprints/BP_MapParent.CoordsToTransform` (`self.MapParent`) (`KismetMathLibrary.FTrunc` _bottomcoord_y) (`KismetMathLibrary.FTrunc` _bottomcoord_x)))
      (`PrimitiveComponent.SetCenterOfMass` (`self.Block`) (* (`KismetMathLibrary.InverseTransformDirection` (`SceneComponent.K2_GetComponentToWorld` (`self.Block`)) (`KismetMathLibrary.Normal` (- (.location _transform_2) (`KismetMathLibrary.MakeVector` _returnvalue_x_2 _returnvalue_y_2)))) 50) "None")
      (`PrimitiveComponent.SetSimulatePhysics` _block_2 true)
      (`PrimitiveComponent.SetCollisionEnabled` _block_2 "QueryAndPhysics"))
    (:`Both`
      (`PrimitiveComponent.SetSimulatePhysics` _block true)
      (`PrimitiveComponent.SetCollisionEnabled` _block "QueryAndPhysics"))))

(fn `isLegal?`
  (returns (Result :type Boolean) (IllegalBlock :type String))
  (locals (String :type String))
  (bind _validtile (`/Game/Tiles/Tile.ValidTile` (`self.TopTile`)))
  (bind _validtile_2 (`/Game/Tiles/Tile.ValidTile` (`self.BottomTile`)))
  (bind _returnvalue (not _validtile))
  (bind _returnvalue_2 (not _validtile_2))
  (if _returnvalue
    (set `self.IllegalBlock` "Top"))
  (if _returnvalue_2
    (set `self.IllegalBlock` "Bottom"))
  (if (and _returnvalue _returnvalue_2)
    (set `self.IllegalBlock` "Both"))
  (return (and _validtile _validtile_2) (`self.IllegalBlock`)))

(fn `ResetBlock`
  (`SceneComponent.K2_DetachFromComponent` (`self.Block`) "KeepWorld" "KeepWorld" "KeepRelative" false)
  (`SceneComponent.K2_SetRelativeLocation` (`self.Root`) (`SceneComponent.K2_GetComponentLocation` (`self.Block`)) false false)
  (`SceneComponent.K2_SetRelativeRotation` :`self` (`self.Pivot`))
  (set `self.Rotating?` false))

(fn `setNewCoordinates`
  (params (`Block Orientation` :type "/Game/Data/E_BlockOrientation Enum" :default "NewEnumerator0") (`Input Direction` :type "/Game/Data/E_Directions Enum" :default "NewEnumerator0"))
  (returns (TopCoord :type "Vector2D Structure") (BottomCoord :type "Vector2D Structure"))
  (bind (_bottomcoord_x _bottomcoord_y) (`KismetMathLibrary.BreakVector2D` (`self.BottomCoord`)))
  (bind (_topcoord_x _topcoord_y) (`KismetMathLibrary.BreakVector2D` (`self.TopCoord`)))
  (bind (_bottomcoord_x_2 _bottomcoord_y_2) (`KismetMathLibrary.BreakVector2D` (`self.BottomCoord`)))
  (bind (_topcoord_x_2 _topcoord_y_2) (`KismetMathLibrary.BreakVector2D` (`self.TopCoord`)))
  (bind (_bottomcoord_x_3 _bottomcoord_y_3) (`KismetMathLibrary.BreakVector2D` (`self.BottomCoord`)))
  (bind (_topcoord_x_3 _topcoord_y_3) (`KismetMathLibrary.BreakVector2D` (`self.TopCoord`)))
  (bind (_bottomcoord_x_4 _bottomcoord_y_4) (`KismetMathLibrary.BreakVector2D` (`self.BottomCoord`)))
  (bind (_topcoord_x_4 _topcoord_y_4) (`KismetMathLibrary.BreakVector2D` (`self.TopCoord`)))
  (bind (_bottomcoord_x_5 _bottomcoord_y_5) (`KismetMathLibrary.BreakVector2D` (`self.BottomCoord`)))
  (bind (_topcoord_x_5 _topcoord_y_5) (`KismetMathLibrary.BreakVector2D` (`self.TopCoord`)))
  (bind (_bottomcoord_x_6 _bottomcoord_y_6) (`KismetMathLibrary.BreakVector2D` (`self.BottomCoord`)))
  (bind (_topcoord_x_6 _topcoord_y_6) (`KismetMathLibrary.BreakVector2D` (`self.TopCoord`)))
  (bind (_topcoord_x_7 _topcoord_y_7) (`KismetMathLibrary.BreakVector2D` (`self.TopCoord`)))
  (bind (_bottomcoord_x_7 _bottomcoord_y_7) (`KismetMathLibrary.BreakVector2D` (`self.BottomCoord`)))
  (bind (_topcoord_x_8 _topcoord_y_8) (`KismetMathLibrary.BreakVector2D` (`self.TopCoord`)))
  (bind (_bottomcoord_x_8 _bottomcoord_y_8) (`KismetMathLibrary.BreakVector2D` (`self.BottomCoord`)))
  (bind (_topcoord_x_9 _topcoord_y_9) (`KismetMathLibrary.BreakVector2D` (`self.TopCoord`)))
  (bind (_bottomcoord_x_9 _bottomcoord_y_9) (`KismetMathLibrary.BreakVector2D` (`self.BottomCoord`)))
  (bind (_topcoord_x_10 _topcoord_y_10) (`KismetMathLibrary.BreakVector2D` (`self.TopCoord`)))
  (bind (_bottomcoord_x_10 _bottomcoord_y_10) (`KismetMathLibrary.BreakVector2D` (`self.BottomCoord`)))
  (bind (_bottomcoord_x_11 _bottomcoord_y_11) (`KismetMathLibrary.BreakVector2D` (`self.BottomCoord`)))
  (bind (_topcoord_x_11 _topcoord_y_11) (`KismetMathLibrary.BreakVector2D` (`self.TopCoord`)))
  (bind (_bottomcoord_x_12 _bottomcoord_y_12) (`KismetMathLibrary.BreakVector2D` (`self.BottomCoord`)))
  (bind (_topcoord_x_12 _topcoord_y_12) (`KismetMathLibrary.BreakVector2D` (`self.TopCoord`)))
  (switch `/Game/Data/E_Directions` `Input Direction`
    (:`NewEnumerator0`
      (switch `/Game/Data/E_BlockOrientation` `Block Orientation`
        (:`NewEnumerator0`
          (set `self.TopCoord` (`KismetMathLibrary.MakeVector2D` _topcoord_x_3 (- _topcoord_y_3 1.0)))
          (set `self.BottomCoord` (`KismetMathLibrary.MakeVector2D` _bottomcoord_x_4 (- _bottomcoord_y_4 2.0))))
        (:`NewEnumerator1`
          (set `self.TopCoord` (`KismetMathLibrary.MakeVector2D` _topcoord_x_2 (- _topcoord_y_2 1.0)))
          (set `self.BottomCoord` (`KismetMathLibrary.MakeVector2D` _bottomcoord_x_3 (- _bottomcoord_y_3 1.0))))
        (:`NewEnumerator2`
          (set `self.TopCoord` (`KismetMathLibrary.MakeVector2D` _topcoord_x (- _topcoord_y 2.0)))
          (set `self.BottomCoord` (`KismetMathLibrary.MakeVector2D` _bottomcoord_x_2 (- _bottomcoord_y_2 1.0))))))
    (:`NewEnumerator1`
      (switch `/Game/Data/E_BlockOrientation` `Block Orientation`
        (:`NewEnumerator0`
          (set `self.TopCoord` (`KismetMathLibrary.MakeVector2D` _topcoord_x_6 (- _topcoord_y_6 -2.0)))
          (set `self.BottomCoord` (`KismetMathLibrary.MakeVector2D` _bottomcoord_x_11 (- _bottomcoord_y_11 -1.0))))
        (:`NewEnumerator1`
          (set `self.TopCoord` (`KismetMathLibrary.MakeVector2D` _topcoord_x_12 (- _topcoord_y_12 -1.0)))
          (set `self.BottomCoord` (`KismetMathLibrary.MakeVector2D` _bottomcoord_x (- _bottomcoord_y -1.0))))
        (:`NewEnumerator2`
          (set `self.TopCoord` (`KismetMathLibrary.MakeVector2D` _topcoord_x_4 (- _topcoord_y_4 -1.0)))
          (set `self.BottomCoord` (`KismetMathLibrary.MakeVector2D` _bottomcoord_x_5 (- _bottomcoord_y_5 -2.0))))))
    (:`NewEnumerator2`
      (switch `/Game/Data/E_BlockOrientation` `Block Orientation`
        (:`NewEnumerator0`
          (set `self.TopCoord` (`KismetMathLibrary.MakeVector2D` (- _topcoord_x_8 1.0) _topcoord_y_8))
          (set `self.BottomCoord` (`KismetMathLibrary.MakeVector2D` (- _bottomcoord_x_8 1.0) _bottomcoord_y_8)))
        (:`NewEnumerator1`
          (set `self.TopCoord` (`KismetMathLibrary.MakeVector2D` (- _topcoord_x_9 1.0) _topcoord_y_9))
          (set `self.BottomCoord` (`KismetMathLibrary.MakeVector2D` (- _bottomcoord_x_9 2.0) _bottomcoord_y_9)))
        (:`NewEnumerator2`
          (set `self.TopCoord` (`KismetMathLibrary.MakeVector2D` (- _topcoord_x_10 2.0) _topcoord_y_10))
          (set `self.BottomCoord` (`KismetMathLibrary.MakeVector2D` (- _bottomcoord_x_10 1.0) _bottomcoord_y_10)))))
    (:`NewEnumerator3`
      (switch `/Game/Data/E_BlockOrientation` `Block Orientation`
        (:`NewEnumerator0`
          (set `self.TopCoord` (`KismetMathLibrary.MakeVector2D` (- _topcoord_x_5 -1.0) _topcoord_y_5))
          (set `self.BottomCoord` (`KismetMathLibrary.MakeVector2D` (- _bottomcoord_x_6 -1.0) _bottomcoord_y_6)))
        (:`NewEnumerator1`
          (set `self.TopCoord` (`KismetMathLibrary.MakeVector2D` (- _topcoord_x_7 -2.0) _topcoord_y_7))
          (set `self.BottomCoord` (`KismetMathLibrary.MakeVector2D` (- _bottomcoord_x_7 -1.0) _bottomcoord_y_7)))
        (:`NewEnumerator2`
          (set `self.TopCoord` (`KismetMathLibrary.MakeVector2D` (- _topcoord_x_11 -1.0) _topcoord_y_11))
          (set `self.BottomCoord` (`KismetMathLibrary.MakeVector2D` (- _bottomcoord_x_12 -2.0) _bottomcoord_y_12))))))
  (return (`self.TopCoord`) (`self.BottomCoord`)))

(fn `UserConstructionScript`)